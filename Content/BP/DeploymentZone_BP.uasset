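; Deployment zone actor that defines a resizable box volume, with no gameplay logic of its own.
; The construction script drives the Box extent from DeploymentSize and raises it by that Z extent so its bottom sits at its parent's origin.
; The StaticMesh is scaled to twice DeploymentSize, matching the box's full dimensions if the mesh is one unit across.
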(fn `UserConstructionScript`
  (bind _box (`self.Box`))
  (bind _deploymentsize (`self.DeploymentSize`))
  (`BoxComponent.SetBoxExtent` _box _deploymentsize true)
  (`SceneComponent.K2_SetRelativeLocation` _box (`KismetMathLibrary.MakeVector` 0.0 0.0 (.z _deploymentsize)) false false)
  (`SceneComponent.SetRelativeScale3D` (`self.StaticMesh`) (* (`self.DeploymentSize`) 2)))